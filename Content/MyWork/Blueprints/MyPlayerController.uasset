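; Player controller for a multiplayer mouse-aimed shooter, bridging input, HUD and the MyGame game mode.
; Right mouse aims and left fires through MyCharacter server calls, with Tick turning the pawn toward the cursor hit and edge-scrolling a detachable camera.
; Damage lowers HealthCurrent, whose RepNotify updates the health bar, and death records frags in the game mode.
; It also handles spawn and respawn requests, a three-player scoreboard and a server file widget.
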(event `InputAction|ThrowGerenade`
  (params (Key :type "Key Structure" :default "AnyKey")))

(event `Key|LeftMouseButton`
  (params (Key :type "Key Structure" :default "AnyKey"))
  (bind _mypawn (`self.MyPawn`))
  ;[1 1 1] Fire
  (:`Pressed`
    (`/Engine/EditorBlueprintResources/ActorMacros.Switch Has Authority`
      (:`Remote`
        (if (`self.Aimed`)
          (bind _mouselocation (`self.GetMouseHitLocation`))
          (bind _asmy_character (cast `/Game/MyWork/Blueprints/MyCharacter` (`self.MyPawn`)))
          (`/Game/MyWork/Blueprints/MyCharacter.FireOnServer` _asmy_character _mouselocation)))))
  (:`Released`
    (`/Engine/EditorBlueprintResources/ActorMacros.Switch Has Authority`
      (:`Remote`
        (`/Engine/EditorBlueprintResources/StandardMacros.IsValid` _mypawn
          (:`Is Valid`
            (bind _asmy_character_2 (cast `/Game/MyWork/Blueprints/MyCharacter` _mypawn))
            (`/Game/MyWork/Blueprints/MyCharacter.FireEndedOnServer` _asmy_character_2)))))))

(event `self.ReceiveBeginPlay`
  ;[1 1 1] Game Initiation on server
  (`/Engine/EditorBlueprintResources/ActorMacros.Switch Has Authority`
    (:`Authority`
      (`self.InitAttributes`)
      (if (not (`KismetSystemLibrary.IsDedicatedServer`))
        (`self.CreateWidgets` :!label _label)
        (`self.SetMouseCursor`)))
    (:`Remote`
      (goto _label))))

(event `Key|RightMouseButton`
  (params (Key :type "Key Structure" :default "AnyKey"))
  ;[1 1 1] Aiming And Facing
  (:`Pressed`
    (set `self.FirstAimHappened` true)
    (set `self.Aimed` true)
    (bind _asmy_character (cast `/Game/MyWork/Blueprints/MyCharacter` (`self.K2_GetPawn`)))
    (set `self.MyPawn` _asmy_character)
    (`/Game/MyWork/Blueprints/MyCharacter.AimOnServer` _asmy_character true))
  (:`Released`
    (set `self.Aimed` false)
    (bind _asmy_character_2 (cast `/Game/MyWork/Blueprints/MyCharacter` (`self.MyPawn`)))
    (`/Game/MyWork/Blueprints/MyCharacter.AimOnServer` _asmy_character_2 false)))

(event `GetFragsFromServer`
  ;[1 1 1] Show Frag
  (`/Engine/EditorBlueprintResources/ActorMacros.Switch Has Authority`
    (:`Authority`
      (bind (_player1kill _player2kill _player3kill _player1death _player2death _player3death) (`self.GetFrags`))
      (`self.ShowFragsOnClient` _player1kill _player2kill _player3kill _player1death _player2death _player3death))))

(event `ShowFragsOnClient`
  (params (Player1Kill :type Text) (Player2Kill :type Text) (Player3Kill :type Text) (Player1Death :type Text) (Player2Death :type Text) (Player3Death :type Text))
  ;[1 1 1] Show Frag
  (`self.ShowFrags` Player1Kill Player2Kill Player3Kill Player1Death Player2Death Player3Death))

(event `self.ReceiveTick`
  (params (DeltaSeconds :type "Float (single-precision)"))
  ;[1 1 1] Aiming And Facing
  (`self.HandleFace`)
  (`self.MoveCameraOnScreenEdge`))

(event `UpdateHealthOnClients`
  ;[1 1 1] Health Control
  (`/Engine/EditorBlueprintResources/ActorMacros.Switch Has Authority`
    (:`Remote`
      (`self.UpdateHealthWidget`))))

(event `RequestRespawnCharacterOnServer`
  (bind _returnvalue (`self.K2_GetPawn`))
  (bind _mygamemodevar (`self.MyGameModeVar`))
  ;[1 1 1] Destroy and Respawn Character
  (`/Engine/EditorBlueprintResources/ActorMacros.Switch Has Authority`
    (:`Authority`
      (`/Engine/EditorBlueprintResources/StandardMacros.IsValid` _returnvalue
        (:`Is Valid`
          (`self.K2_DestroyActor` _returnvalue))
        (:`Is Not Valid`
          _))
      (`self.RemoveGamePlayAttributes`)
      (`/Engine/EditorBlueprintResources/StandardMacros.IsValid` _mygamemodevar
        (:`Is Valid`
          (bind _asmy_game (cast `/Game/MyWork/Blueprints/MyGame` _mygamemodevar))
          (`/Engine/EditorBlueprintResources/StandardMacros.IsValid` _asmy_game
            (:`Is Valid`
              (`/Game/MyWork/Blueprints/MyGame.RespawnCharacterOnServer` _asmy_game self (`self.PlayerIndex`)))))))))

(event `UpdateHealthOnServer`
  (params (Damage :type "Float (double-precision)") (ShooterIndex :type Integer))
  ;[1 1 1] Health Control
  (bind _output_get (set `self.HealthCurrent` (- (`self.HealthCurrent`) Damage)))
  (if (<= _output_get 0.0)
    (bind _asmy_game (cast `/Game/MyWork/Blueprints/MyGame` (`self.MyGameModeVar`)))
    (`/Game/MyWork/Blueprints/MyGame.AddKillToPlayer` _asmy_game ShooterIndex)
    (`/Game/MyWork/Blueprints/MyGame.AddDeathToPlayer` _asmy_game (`self.PlayerIndex`))
    (bind _asmy_character (cast `/Game/MyWork/Blueprints/MyCharacter` (`self.MyPawn`)))
    (`/Game/MyWork/Blueprints/MyCharacter.DeathOnServer` _asmy_character)))

(event `RemoveGamePlayAttributes`
  (bind _myhealthbar (`self.MyHealthbar`))
  ;[1 1 1] Destroy and Respawn Character
  (`/Engine/EditorBlueprintResources/StandardMacros.IsValid` _myhealthbar
    (:`Is Valid`
      (`Widget.RemoveFromParent` _myhealthbar))))

(event `InputAction|ServerSaveMenu`
  (params (Key :type "Key Structure" :default "AnyKey"))
  ;[1 1 1] Server File Handle
  (:`Pressed`
    (if (`self.ServerFileMode`)
      (`Widget.RemoveFromParent` (`self.ServerFileWidget`))
      (set `self.ServerFileMode` false)
      (else
        (bind _returnvalue (`|CreateWidget` "/Game/MyWork/Blueprints/InputCommand.InputCommand_C" self))
        (bind _output_get (set `self.ServerFileWidget` _returnvalue))
        (`UserWidget.AddToViewport` _output_get 0)
        (set `self.ServerFileMode` true)))))

(event `RequestSpawnCharacterOnServer`
  ;[1 1 1] Spawn Character
  (bind _asmy_game (cast `/Game/MyWork/Blueprints/MyGame` (`GameplayStatics.GetGameMode`)))
  (`/Game/MyWork/Blueprints/MyGame.CreateNewCharacter` _asmy_game self))

(fn `AttemptAim`
  (`/Engine/EditorBlueprintResources/ActorMacros.Switch Has Authority`
    (:`Authority`
      (set `self.Aimed` true))))

(fn `AttemptNotAim`
  (`/Engine/EditorBlueprintResources/ActorMacros.Switch Has Authority`
    (:`Authority`
      (set `self.Aimed` false))))

(fn `CreateWidgets`
  (set `self.ViewPortSize` (`WidgetLayoutLibrary.GetViewportSize`))
  (bind _returnvalue (`|CreateWidget` "/Game/MyWork/Blueprints/MyMenuOnScreen.MyMenuOnScreen_C" self))
  (`UserWidget.AddToViewport` _returnvalue 0))

(fn `FindPlayerIndex`
  (params (InputCharacter :type "Actor Object Reference"))
  (bind _outactors (`GameplayStatics.GetAllActorsOfClass` "/Game/MyWork/Blueprints/MyCharacter.MyCharacter_C"))
  (for _ _outactors
    _))

(fn `GetFaceRotation`
  (returns (RotateToCursor :type "Rotator Structure"))
  (bind _mouselocation (`self.GetMouseHitLocation`))
  (return (`KismetMathLibrary.MakeRotator` 0.0 0.0 (.yaw (`KismetMathLibrary.FindLookAtRotation` (`self.K2_GetActorLocation`) _mouselocation)))))

(fn `GetFrags`
  (returns (Player1Kill :type Text) (Player2Kill :type Text) (Player3Kill :type Text) (Player1Death :type Text) (Player2Death :type Text) (Player3Death :type Text))
  (`/Engine/EditorBlueprintResources/ActorMacros.Switch Has Authority`
    (:`Authority`
      (bind _asmy_game (cast `/Game/MyWork/Blueprints/MyGame` (`GameplayStatics.GetGameMode`))
        (:`then`
          _)
        (:`CastFailed`
          (`KismetSystemLibrary.PrintString` "cast to mygame failed in show frags" true false (struct :`G` 0.66 :`B` 1.0 :`A` 1.0) 12.0))))
    (:`Remote`
      _))
  (bind _playerkill (`/Game/MyWork/Blueprints/MyGame.PlayerKill` _asmy_game))
  (bind _playerdeath (`/Game/MyWork/Blueprints/MyGame.PlayerDeath` _asmy_game))
  (return (`KismetTextLibrary.Conv_IntToText` (`KismetArrayLibrary.Array_Get` _playerkill)) (`KismetTextLibrary.Conv_IntToText` (`KismetArrayLibrary.Array_Get` _playerkill 1)) (`KismetTextLibrary.Conv_IntToText` (`KismetArrayLibrary.Array_Get` _playerkill 2)) (`KismetTextLibrary.Conv_IntToText` (`KismetArrayLibrary.Array_Get` _playerdeath)) (`KismetTextLibrary.Conv_IntToText` (`KismetArrayLibrary.Array_Get` _playerdeath 1)) (`KismetTextLibrary.Conv_IntToText` (`KismetArrayLibrary.Array_Get` _playerdeath 2))))

(fn `GetMouseHitLocation`
  (returns (MouseLocation :type "Vector Structure"))
  (return (`.Location` (`GameplayStatics.BreakHitResult` (`self.GetHitResultUnderCursorByChannel` "TraceTypeQuery1" true)))))

(fn `HandleFace`
  (if (`self.FirstAimHappened`)
    (if (`self.Aimed`)
      (bind _rotatetocursor (`self.GetFaceRotation`))
      (bind _asmy_character (cast `/Game/MyWork/Blueprints/MyCharacter` (`self.MyPawn`)))
      (`/Game/MyWork/Blueprints/MyCharacter.FaceOnServer` _asmy_character _rotatetocursor))))

(fn `HideFrags`
  (bind _myfrag (`self.MyFrag`))
  (`/Engine/EditorBlueprintResources/StandardMacros.IsValid` _myfrag
    (:`Is Valid`
      (`Widget.RemoveFromParent` _myfrag))))

(fn `InitAttributes`
  (`self.InitBullets`)
  (`self.InitLevelAndGameVar`))

(fn `InitBullets`
  (set `self.HasBullet` true))

(fn `InitLevelAndGameVar`
  (bind _returnvalue (`GameplayStatics.GetCurrentLevelName` true))
  (bind _output_get (set `self.MyGameModeVar` (`GameplayStatics.GetGameMode`)))
  (bind _asmy_game (cast `/Game/MyWork/Blueprints/MyGame` _output_get))
  (set `/Game/MyWork/Blueprints/MyGame.LevelPlaying` (`KismetStringLibrary.Conv_StringToName` _returnvalue) _asmy_game))

(fn `MoveCameraOnScreenEdge`
  (locals (XVector :type "Float (double-precision)") (YVector :type "Float (double-precision)") (XMouse :type "Float (double-precision)") (YMouse :type "Float (double-precision)") (EdgeLimit :type "Float (double-precision)" :default 20.0) (ScrollValue :type "Float (double-precision)" :default 20.0))
  (bind (_locationx _locationy) (`self.GetMousePosition`))
  (bind _mypawn (`self.MyPawn`))
  (bind _xmouse (`local.XMouse`))
  (bind _ymouse (`local.YMouse`))
  (bind _edgelimit (`local.EdgeLimit`))
  (bind _scrollvalue (`local.ScrollValue`))
  (bind (_x _y) (`KismetMathLibrary.BreakVector2D` (`WidgetLayoutLibrary.GetViewportSize`)))
  (bind _returnvalue (* -1 _scrollvalue))
  (bind _returnvalue_2 (- _x (`local.XMouse`)))
  (bind _returnvalue_3 (- _y (`local.YMouse`)))
  (bind _returnvalue_4 (and (< _xmouse _edgelimit) (> _xmouse 0.0)))
  (bind _returnvalue_5 (and (< _returnvalue_2 _edgelimit) (> _returnvalue_2 0.0)))
  (`/Engine/EditorBlueprintResources/ActorMacros.Switch Has Authority`
    (:`Remote`
      (set `local.XMouse` _locationx)
      (set `local.YMouse` _locationy)
      (if _returnvalue_4
        (set `local.XVector` _scrollvalue)
        (set `local.YVector` _returnvalue)
        (elif _returnvalue_5
          (set `local.XVector` _returnvalue)
          (set `local.YVector` _scrollvalue)))
      (if (and (< _ymouse _edgelimit) (> _ymouse 0.0))
        (set `local.YVector` _scrollvalue)
        (set `local.XVector` _scrollvalue)
        (`/Engine/EditorBlueprintResources/StandardMacros.IsValid` _mypawn :!label _label
          (:`Is Valid`
            (bind _asmy_character (cast `/Game/MyWork/Blueprints/MyCharacter` _mypawn))
            (if (`/Game/MyWork/Blueprints/MyCharacter.IsCameraCentre` _asmy_character)
              (set `/Game/MyWork/Blueprints/MyCharacter.IsCameraCentre` false _asmy_character)
              (`SceneComponent.DetachFromParent` (`/Game/MyWork/Blueprints/MyCharacter.Camera` _asmy_character) true true))
            (`/Game/MyWork/Blueprints/MyCharacter.MoveCamera` _asmy_character (`KismetMathLibrary.MakeVector` (`local.XVector`) (`local.YVector`) 0.0))))
        (elif (and (< _returnvalue_3 _edgelimit) (> _returnvalue_3 0.0))
          (set `local.YVector` _returnvalue)
          (set `local.XVector` _returnvalue)
          (goto _label)
          (elif (or _returnvalue_4 _returnvalue_5)
            (goto _label)))))))

(fn `OnRep_HasBullet`)

(fn `OnRep_HealthCurrent`
  (`self.UpdateHealthOnClients`))

(fn `SetMouseCursor`
  (bind _returnvalue (`GameplayStatics.GetCurrentLevelName` true))
  (if (`KismetStringLibrary.EqualEqual_StrStr` _returnvalue "Entry")
    (set `self.CurrentMouseCursor` "Default")
    (else
      (set `self.CurrentMouseCursor` "Crosshairs"))))

(fn `ShowFrags`
  (params (Player1Kill :type Text) (Player2Kill :type Text) (Player3Kill :type Text) (Player1Death :type Text) (Player2Death :type Text) (Player3Death :type Text))
  (bind _returnvalue (`|CreateWidget` "/Game/MyWork/Blueprints/Frags.Frags_C" self))
  (bind _output_get (set `self.MyFrag` _returnvalue))
  (`TextBlock.SetText` (`/Game/MyWork/Blueprints/Frags.Player1Kill` _output_get) Player1Kill)
  (`TextBlock.SetText` (`/Game/MyWork/Blueprints/Frags.Player2Kill` _output_get) Player2Kill)
  (`TextBlock.SetText` (`/Game/MyWork/Blueprints/Frags.Player3Kill` _output_get) Player3Kill)
  (`TextBlock.SetText` (`/Game/MyWork/Blueprints/Frags.Player1Death` _output_get) Player1Death)
  (`TextBlock.SetText` (`/Game/MyWork/Blueprints/Frags.Player2Death` _output_get) Player2Death)
  (`TextBlock.SetText` (`/Game/MyWork/Blueprints/Frags.Player3Death` _output_get) Player3Death)
  (`UserWidget.AddToViewport` _output_get 0))

(fn `UpdateHealthWidget`
  (bind _myhealthbar (`self.MyHealthbar`))
  (`/Engine/EditorBlueprintResources/StandardMacros.IsValid` _myhealthbar
    (:`Is Valid`
      (bind _asmy_screen_health_bar (cast `/Game/MyWork/Blueprints/MyScreenHealthBar` _myhealthbar)
        (:`then`
          (`ProgressBar.SetPercent` (`/Game/MyWork/Blueprints/MyScreenHealthBar.VerticalHealth` _asmy_screen_health_bar) (/ (`self.HealthCurrent`) 100.0)))
        (:`CastFailed`
          (`KismetSystemLibrary.PrintString` "cast to my screen health failed" true true (struct :`G` 0.66 :`B` 1.0 :`A` 1.0) 8.0))))))

(fn `UserConstructionScript`)
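; MyGrenade is a grenade that damages a living character other than its shooter on overlap.
; Overlaps pass to an authority-only handler, which uses HitAnyCharacter to validate the target, excluding the shooter by display-name comparison.
; A valid hit applies damage with the shooter as causer and calls SpawnParticleEverywhere to play an explosion at the target's location.
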(event Custom|AttemptHitOnServer
  (params (HitActor :type Actor%20Object%20Reference))
  ;[1 1 1] Apply Damage on Hit
  (Game|Damage|ApplyDamage HitActor (Variables|Attributes|GetDamage) 0 (Variables|Shooter|GetShooterCharacter)))

(event Custom|SpawnParticleEverywhere
  (params (Object :type Actor%20Object%20Reference))
  ;[1 1 1] Show hit effects
  (Effects|SpawnEmitteratLocation (Variables|Effects|GetExplosionEffect) (Transformation|GetActorLocation Object)))

(event Collision|EventActorBeginOverlap
  (params (OtherActor :type Actor%20Object%20Reference))
  ;[1 1 1] Handle Overlap
  (CallFunction|HandleOverlaponServer OtherActor))

(fn ConstructionScript)

(fn HitAnyCharacter
  (params (Object :type Actor%20Object%20Reference))
  (bind _returnvalue (Utilities|GetDisplayName Object))
  (bind _shootercharacter (Variables|Shooter|GetShooterCharacter))
  (bind _returnvalue_2 (Utilities|GetDisplayName _shootercharacter))
  (Utilities|IsValid Object
    (:Is%20Valid
      (bind _asmy_character (Utilities|Casting|CastToMyCharacter Object)
        (:then
          (if (and (Utilities|Enum|NotEqual(Enum) _returnvalue _returnvalue_2) (Variables|/Game/MyWork/Blueprints/MyCharacter.MyCharacter_C|GetIsAlive _asmy_character))
            (LocalVariables|SetIsHitting true)
            (Development|PrintString (Utilities|String|BuildString(Name) (Utilities|String|BuildString(Name) "" "Shooter: " (Utilities|String|StringToName _returnvalue_2) " ") "Shot: " (Utilities|String|StringToName _returnvalue) "") true false "(R=0.000000,G=0.660000,B=1.000000,A=1.000000)" 8.0)
            (else
              (LocalVariables|SetIsHitting false))))
        (:CastFailed
          (Development|PrintString "cast to my character failed in hitanycharacter" true false "(R=0.000000,G=0.660000,B=1.000000,A=1.000000)" 8.0)
          (LocalVariables|SetIsHitting false))))
    (:Is%20Not%20Valid
      _))
  (return (LocalVariables|GetIsHitting)))

(fn HandleOverlaponServer
  (params (Object :type Actor%20Object%20Reference))
  (Networking|SwitchHasAuthority
    (:Authority
      (Utilities|IsValid (Variables|Shooter|GetShooterCharacter)
        (:Is%20Valid
          (bind _hits (CallFunction|HitAnyCharacter Object))
          (if _hits
            (CallFunction|AttemptHitonServer Object)
            (CallFunction|SpawnParticleEverywhere Object)))))))
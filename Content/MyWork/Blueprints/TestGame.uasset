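; TestGame is a test Blueprint that exercises breaking out of a for-each loop and prints debug results.
; On BeginPlay it searches an array for an element equal to a comparison variable.
; On a match it calls the BrakeLoop custom event, which triggers the loop's break, then prints the comparison result.
; After the loop it prints the current array element.
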(event `self.ReceiveBeginPlay`
  (for _array_element (`self.NewVar_0`) :!label _label
    (bind _returnvalue (== _array_element (`self.NewVar_1`)))
    (if _returnvalue
      (`self.BrakeLoop`)
      (`KismetSystemLibrary.PrintString` (`KismetStringLibrary.Conv_BoolToString` _returnvalue) true false (struct :`G` 0.66 :`B` 1.0 :`A` 1.0) 12.0)))
  (`KismetSystemLibrary.PrintString` (`KismetStringLibrary.Conv_IntToString` _array_element) true false (struct :`G` 0.66 :`B` 1.0 :`A` 1.0) 12.0))

(event `BrakeLoop`
  (goto _label :!via `Break`))

(fn `UserConstructionScript`)